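; Robot arm actor Blueprint that rotates its skeletal mesh a quarter turn in yaw on demand.
; Pressing U calls RotateRbot, which stores the mesh's current relative rotation as the start.
; A timeline then lerps from that rotation to the start combined with a 90-degree yaw, taking the shortest path.
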(event `RotateRbot`
  ;[1 1 1] RotationEvent
  (bind _output_get (set `self.StartRotation` (`SceneComponent.RelativeRotation` (`self.SkeletalMesh`))))
  (bind (_direction _robotrotation) (`Timeline|Timeline_0` :!via `PlayFromStart`)
    (:`Update`
      (`SceneComponent.K2_SetRelativeRotation` (`self.SkeletalMesh`) (`KismetMathLibrary.RLerp` (`self.StartRotation`) (`KismetMathLibrary.ComposeRotators` _output_get (`KismetMathLibrary.MakeRotator` 0.0 0.0 90.0)) _robotrotation true) false false))))

(event `Key|U`
  (params (Key :type "Key Structure"))
  (:`Pressed`
    (`self.RotateRbot`)))

(fn `UserConstructionScript`)