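; Phone actor whose spotlight, hidden at BeginPlay, is switched by a boolean from the game server actor.
; At startup it adds a JSONComponent with the activateLightsTrigger ID, defaulted to false, and attaches it to the GameServerActor.
; The component's value-change event reads the boolean back and applies it to the light's visibility, printing debug messages along the way.
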(event `self.ReceiveBeginPlay`
  (`SceneComponent.SetVisibility` (`self.SpotLight`) false false)
  (bind _returnvalue (`AddComponent|NODE_AddJSONComponent-0`))
  (set `JSONComponent.id` "\"activateLightsTrigger\"" _returnvalue)
  (`JSONComponent.setValueBool` _returnvalue false)
  (bind _returnvalue_2 (`GameplayStatics.GetActorOfClass` "/Script/MyProject.GameServerActor"))
  (`GameServerActor.attach` _returnvalue_2 _returnvalue)
  (add `JSONComponent.OnValueChanged` _returnvalue (delegate `OnValueChanged_Event_1`)))

(event `ActivatePhoneLight`
  ;[1 1 1] Activate Phone Light
  (bind _returnvalue (`JSONComponent.getValueBool` (`self.GetComponentByClass` "/Script/MyProject.JSONComponent")))
  (`KismetSystemLibrary.PrintString` (`KismetStringLibrary.Conv_BoolToString` _returnvalue))
  (`SceneComponent.SetVisibility` (`self.SpotLight`) _returnvalue false))

(event `OnValueChanged_Event_1`
  (`KismetSystemLibrary.PrintString` "Switch!")
  (`self.ActivatePhoneLight`))

(fn `UserConstructionScript`)