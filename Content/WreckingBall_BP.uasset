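; Wrecking ball Blueprint whose Base the player slides along X and Y with the numpad.
; Keys 8/2 and 4/6 set X and Y speed, and 5 stops both.
; Tick moves Base by a frame-rate-dependent step while it overlaps that axis's collision, stays within fixed bounds, and the other axis speed is zero.
; A timeline-based X move remains as an event named OLD, not called here.
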(event `Key|NumPadEight`
  (params (Key :type "Key Structure"))
  ;[1 1 1] Set Speeds
  (:`Pressed`
    (set `self.X Speed` -1.0)))

(event `Key|NumPadTwo`
  (params (Key :type "Key Structure"))
  ;[1 1 1] Set Speeds
  (:`Pressed`
    (set `self.X Speed` 1.0)))

(event `Key|NumPadFive`
  (params (Key :type "Key Structure"))
  ;[1 1 1] Set Speeds
  (:`Pressed`
    (set `self.X Speed` 0.0)
    (set `self.Y Speed` 0.0)))

(event `self.ReceiveTick`
  (params (DeltaSeconds :type "Float (single-precision)"))
  (bind _base (`self.Base`))
  (if (`PrimitiveComponent.IsOverlappingComponent` (`self.YAxisCollision`) _base)
    (`self.OnMoveYAxis`))
  (if (`PrimitiveComponent.IsOverlappingComponent` (`self.XAxisCollision`) _base)
    (`self.OnMoveXAxis`)))

(event `Key|NumPadFour`
  (params (Key :type "Key Structure"))
  ;[1 1 1] Set Speeds
  (:`Pressed`
    (set `self.Y Speed` -1.0)))

(event `Key|NumPadSix`
  (params (Key :type "Key Structure"))
  ;[1 1 1] Set Speeds
  (:`Pressed`
    (set `self.Y Speed` 1.0)))

(event `OnMoveYAxis`
  (bind _base (`self.Base`))
  (bind _y (.y (`SceneComponent.RelativeLocation` (`self.Base`))))
  ;[1 1 1] Move on Y Axis
  (if (and (<= _y 1000.0) (>= _y -1000.0))
    (if (== (`self.X Speed`) 0.0)
      (`SceneComponent.K2_AddRelativeLocation` _base (* (`SceneComponent.GetRightVector` _base) (* 3 (`self.Y Speed`))) false false))))

(event `OnMoveXAxis`
  (bind _base (`self.Base`))
  (bind _x (.x (`SceneComponent.RelativeLocation` (`self.Base`))))
  ;[1 1 1] Move on X Axis
  (if (and (<= _x 500.0) (>= _x -500.0))
    (if (== (`self.Y Speed`) 0.0)
      (`SceneComponent.K2_AddRelativeLocation` _base (`KismetMathLibrary.ClampVectorSize` (* (`SceneComponent.GetForwardVector` _base) (* 3 (`self.X Speed`))) -450.0 450.0) false false))))

(event `OLD`
  (bind _base (`self.Base`))
  ;[1 1 1] Move On X Axis To Position (Old)
  (bind _output_get (set `self.Start Position` (`SceneComponent.RelativeLocation` _base)))
  (bind (_direction _xposition) (`Timeline|WreckingBallTimeLineX` :!via `PlayFromStart`)
    (:`Update`
      (`SceneComponent.K2_SetRelativeLocation` _base (`KismetMathLibrary.VLerp` _output_get (+ _output_get (`KismetMathLibrary.MakeVector` (`self.X Speed`))) _xposition) false false))))

(fn `UserConstructionScript`)